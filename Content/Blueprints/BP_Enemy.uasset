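; BP_Enemy is an enemy pawn that moves toward the first player's pawn through AI movement.
; After a short delay on BeginPlay, it issues a single AIMoveTo that targets the player with an acceptance radius.
; An unconnected branch that never runs would attach the first BP_Axe in the level to the left-hand socket, then start the same move.
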(event `self.ReceiveBeginPlay`
  (`KismetSystemLibrary.Delay` 2.0)
  (`|AIMoveTo` self (0.0 0.0 0.0) (`GameplayStatics.GetPlayerPawn` 0) 150.0))

(fn `UserConstructionScript`)