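; Elevator actor that moves its platform mesh vertically, starting automatically at BeginPlay.
; A Timeline sets the platform's relative Z from its alpha times MaxZ, printing that height on each update.
; The trigger volume registers or clears this elevator as OverlapElevator on the player's BP_ThirdPersonCharacter.
; Tick does nothing effective, and the offset, direction-change and hide logic is left unconnected in the event graph.
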(event `self.ReceiveBeginPlay`
  (bind (_direction _alpha) (`Timeline|Timeline` :!via `PlayFromStart`)
    (:`Update`
      (bind _returnvalue (* _alpha (`self.MaxZ`)))
      (`KismetSystemLibrary.PrintString` (`KismetStringLibrary.Conv_DoubleToString` _returnvalue))
      (`SceneComponent.K2_SetRelativeLocation` (`self.PlatformMesh`) (`KismetMathLibrary.MakeVector` 0.0 0.0 _returnvalue) false false))))

(event `self.ReceiveTick`
  (params (DeltaSeconds :type "Float (single-precision)"))
  (if (`self.PlayElevator`)
    _))

(event `self.PlatformTrigger.OnComponentBeginOverlap`
  (params (OverlappedComponent :type "PrimitiveComponent Object Reference") (OtherActor :type "Actor Object Reference") (OtherComp :type "PrimitiveComponent Object Reference") (OtherBodyIndex :type Integer) (bFromSweep :type Boolean) (SweepResult :type "HitResult Structure (by ref)"))
  (bind _returnvalue (`GameplayStatics.GetPlayerPawn` 0))
  (if (== OtherActor _returnvalue)
    (bind _asbp_third_person_character (cast `/Game/ThirdPerson/Blueprints/BP_ThirdPersonCharacter` _returnvalue))
    (set `/Game/ThirdPerson/Blueprints/BP_ThirdPersonCharacter.OverlapElevator` self _asbp_third_person_character)))

(event `self.PlatformTrigger.OnComponentEndOverlap`
  (params (OverlappedComponent :type "PrimitiveComponent Object Reference") (OtherActor :type "Actor Object Reference") (OtherComp :type "PrimitiveComponent Object Reference") (OtherBodyIndex :type Integer))
  (bind _returnvalue (`GameplayStatics.GetPlayerPawn` 0))
  (if (== OtherActor _returnvalue)
    (bind _asbp_third_person_character (cast `/Game/ThirdPerson/Blueprints/BP_ThirdPersonCharacter` _returnvalue))
    (set `/Game/ThirdPerson/Blueprints/BP_ThirdPersonCharacter.OverlapElevator` null _asbp_third_person_character)))

(fn `AddZOffset`
  (params (Offset :type "Float (double-precision)")))

(fn `ChangeDirection`
  (set `self.DeltaZ` (* (`self.DeltaZ`) -1.0)))

(fn `Hide`
  (`SceneComponent.SetHiddenInGame` (`self.DefaultSceneRoot`) true true))

(fn `ShouldChangeDirection`
  (returns (ReturnValue :type Boolean))
  (bind (_relativelocation_x _relativelocation_y _relativelocation_z) (`KismetMathLibrary.BreakVector` (`SceneComponent.RelativeLocation` (`self.PlatformMesh`))))
  (return (or (>= _relativelocation_z (`self.MaxZ`)) (<= _relativelocation_z 0.0))))

(fn `Show`
  (`SceneComponent.SetHiddenInGame` (`self.PlatformMesh`) false true))

(fn `UserConstructionScript`)