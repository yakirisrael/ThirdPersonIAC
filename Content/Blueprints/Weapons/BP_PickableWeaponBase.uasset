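; Base pickup actor for axe, sword or bow weapons that the player collects by walking into it.
; On BeginPlay it sets its static mesh from the weapon Type and caches the third-person game mode.
; When the player overlaps the capsule, it adds the Type to the character's collected weapons, has the UI manager show a message and swap the HUD weapon image, then destroys itself.
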(event `self.ReceiveBeginPlay`
  (`StaticMeshComponent.SetStaticMesh` (`self.StaticMesh`) (select `/Game/Enums/E_WeaponType` (`self.Type`) :`NewEnumerator0` "/Game/LP_RPGWeapons_JC/Models/SM_Ax_01.SM_Ax_01" :`NewEnumerator1` "/Game/LP_RPGWeapons_JC/Models/SM_Sword_01.SM_Sword_01" :`NewEnumerator2` "/Game/LP_RPGWeapons_JC/Models/SM_Bow_01.SM_Bow_01" :!type "StaticMesh Object Reference"))
  (bind _asbp_third_person_game_mode (cast `/Game/ThirdPerson/Blueprints/BP_ThirdPersonGameMode` (`GameplayStatics.GetGameMode`)))
  (set `self.As BP Third Person Game Mode` _asbp_third_person_game_mode))

(event `self.Capsule.OnComponentBeginOverlap`
  (params (OverlappedComponent :type "PrimitiveComponent Object Reference") (OtherActor :type "Actor Object Reference") (OtherComp :type "PrimitiveComponent Object Reference") (OtherBodyIndex :type Integer) (bFromSweep :type Boolean) (SweepResult :type "HitResult Structure (by ref)"))
  (bind _returnvalue (`GameplayStatics.GetPlayerPawn` 0))
  (bind _ui_manager (`/Game/ThirdPerson/Blueprints/BP_ThirdPersonGameMode.UI Manager` (`self.As BP Third Person Game Mode`)))
  (if (== OtherActor _returnvalue)
    (bind _asbp_third_person_character (cast `/Game/ThirdPerson/Blueprints/BP_ThirdPersonCharacter` _returnvalue))
    (bind _weaponscollected (`/Game/ThirdPerson/Blueprints/BP_ThirdPersonCharacter.WeaponsCollected` _asbp_third_person_character))
    (`KismetArrayLibrary.Array_Add` _weaponscollected (`self.Type`))
    (for _ _weaponscollected
      _)
    (`|ExecutionSequence`
      (:`then_0`
        (`/Game/UI/BP_UIManager.Show Weapon Added Message` _ui_manager (`self.Type`))
        (`/Game/UI/HUD.ReplaceWeaponImage` (`/Game/UI/BP_UIManager.HUD` _ui_manager) (`self.Type`)))
      (:`then_1`
        (`self.K2_DestroyActor`)))))

(fn `UserConstructionScript`)